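; Player controller for the space shooter that spawns and possesses the player ship, then switches the view to the level's BP_Camera.
; Movement axes push the ship along the X and Z plane scaled by its Speed, and the launch action fires its laser.
; Every tick, SetBoundary clamps the ship's position to a fixed rectangle in X and Z by resetting its location.
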(event `self.ReceiveBeginPlay`
  (bind _returnvalue (`|SpawnActorFromClass` "/Game/SpaceShooter/Gameplay/BP_PlayerShip.BP_PlayerShip_C" (`KismetMathLibrary.MakeTransform` (0.0 1.0 0.0)) "AlwaysSpawn" "OverrideRootScale" null null))
  (bind _output_get (set `self.PlayerShip` _returnvalue))
  (`self.Possess` _output_get)
  (bind _returnvalue_2 (`GameplayStatics.GetActorOfClass` "/Game/SpaceShooter/Gameplay/BP_Camera.BP_Camera_C"))
  (`self.SetViewTargetWithBlend` _returnvalue_2))

(event `InputAxis|MoveDown`
  (params (AxisValue :type "Float (single-precision)"))
  (if (!= AxisValue 0.0)
    (`/Engine/EditorBlueprintResources/StandardMacros.IsValid` (`self.PlayerShip`)
      (:`Is Valid`
        (`Pawn.AddMovementInput` (`self.PlayerShip`) (`KismetMathLibrary.MakeVector` 0.0 0.0 (* (`/Game/SpaceShooter/Gameplay/BP_Master_Ship.Speed` (`self.PlayerShip`)) AxisValue)) 1.0 false)))))

(event `InputAxis|MoveRight`
  (params (AxisValue :type "Float (single-precision)"))
  (if (!= AxisValue 0.0)
    (`/Engine/EditorBlueprintResources/StandardMacros.IsValid` (`self.PlayerShip`)
      (:`Is Valid`
        (`Pawn.AddMovementInput` (`self.PlayerShip`) (`KismetMathLibrary.MakeVector` (* AxisValue (`/Game/SpaceShooter/Gameplay/BP_Master_Ship.Speed` (`self.PlayerShip`)))) 1.0 false)))))

(event `self.ReceiveTick`
  (params (DeltaSeconds :type "Float (single-precision)"))
  (`self.SetBoundary`))

(event `InputAction|launch`
  (params (Key :type "Key Structure"))
  (:`Pressed`
    (`/Engine/EditorBlueprintResources/StandardMacros.IsValid` (`self.PlayerShip`)
      (:`Is Valid`
        (`/Game/SpaceShooter/Gameplay/BP_Master_Ship.LaunchLaser` (`self.PlayerShip`))))))

(fn `SetBoundary`
  (bind _returnvalue (`self.K2_GetActorLocation` (`self.PlayerShip`)))
  (bind _returnvalue_2 (`self.K2_GetActorLocation` (`self.PlayerShip`)))
  (`/Engine/EditorBlueprintResources/StandardMacros.IsValid` (`self.PlayerShip`)
    (:`Is Valid`
      (if (> (.x _returnvalue) 1024.0)
        (`self.K2_SetActorLocation` (`self.PlayerShip`) (`KismetMathLibrary.MakeVector` 1024.0 (.y _returnvalue) (.z _returnvalue)) false false))
      (if (< (.x _returnvalue) -1024.0)
        (`self.K2_SetActorLocation` (`self.PlayerShip`) (`KismetMathLibrary.MakeVector` -1024.0 (.y _returnvalue) (.z _returnvalue)) false false))
      (if (< (.z _returnvalue_2) -500.0)
        (`self.K2_SetActorLocation` (`self.PlayerShip`) (`KismetMathLibrary.MakeVector` (.x _returnvalue_2) (.y _returnvalue_2) -500.0) false false))
      (if (> (.z _returnvalue_2) 500.0)
        (`self.K2_SetActorLocation` (`self.PlayerShip`) (`KismetMathLibrary.MakeVector` (.x _returnvalue_2) (.y _returnvalue_2) 500.0) false false)))))

(fn `UserConstructionScript`)