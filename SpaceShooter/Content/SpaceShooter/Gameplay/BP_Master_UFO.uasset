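; Master UFO enemy Blueprint for the space shooter that descends along Z and can drop an item when destroyed.
; Move offsets X around the spawn position with a sine wave driven by current height.
; On Destroyed, a probability roll spawns a class picked by RandomItemByWidget from a weight map.
; That pick compares against a fixed 0–0 random range, so it returns the first non-negative-weight entry instead of a weighted choice.
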(event `self.ReceiveBeginPlay`
  (`parent.ReceiveBeginPlay`)
  (set `self.PositionX` (.x (`self.K2_GetActorLocation`))))

(event `self.ReceiveDestroyed`
  (if (>= (`self.DropProbability`) (`KismetMathLibrary.RandomIntegerInRange` 0 10000))
    (`|SpawnActorFromClass` (`self.RandomItemByWidget`) (`self.GetTransform`) "AlwaysSpawn" "OverrideRootScale" null null)))

(fn `Move`
  (params (delta :type "Float (double-precision)"))
  (locals (waveFrequency :type "Float (double-precision)" :default 5.0) (waveWidth :type "Float (double-precision)" :default 200.0))
  (bind _z (.z (`self.K2_GetActorLocation`)))
  (`self.K2_SetActorLocation` (`KismetMathLibrary.MakeVector` (+ (`self.PositionX`) (* (`local.waveWidth`) (`KismetMathLibrary.DegSin` (* (`KismetMathLibrary.GetPI`) 2.0 (/ _z (`local.waveFrequency`)))))) (.y (`self.K2_GetActorLocation`)) (- _z (* delta (`self.Speed`))))))

(fn `RandomItemByWidget`
  (returns (SpawnClass :type "Actor Class Reference"))
  (locals (Widget :type Integer :default 0) (WidgetTotal :type Integer :default 0))
  (set `local.Widget` 0)
  (bind _values (`BlueprintMapLibrary.Map_Values` (`self.Enemies Random Weight`)))
  (for _array_element _values
    (set `local.WidgetTotal` (+ (`local.WidgetTotal`) _array_element)))
  (bind _values_2 (`BlueprintMapLibrary.Map_Values` (`self.Enemies Random Weight`)))
  (for (_array_element_2 _array_index) _values_2
    (if (>= _array_element_2 (`KismetMathLibrary.RandomIntegerInRange` 0))
      (bind _keys (`BlueprintMapLibrary.Map_Keys` (`self.Enemies Random Weight`)))
      (return (`|GetArrayItem` _keys _array_index))
      (else
        (set `local.Widget` (+ _array_element_2 (`local.Widget`)))))))

(fn `UserConstructionScript`
  (`parent.UserConstructionScript`))