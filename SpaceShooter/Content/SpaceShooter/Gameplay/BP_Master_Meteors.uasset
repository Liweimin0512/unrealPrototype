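; BP_Master_Meteors is a meteor actor for the space shooter, named as a master Blueprint and drawn with a Paper2D sprite.
; The construction script applies the Sprite variable to the sprite component.
; Tick moves it down world Z by Speed scaled by delta time and adds pitch spin proportional to Speed per frame, without delta scaling.
; It destroys itself once it falls to a fixed lower Z limit.
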(event `self.ReceiveTick`
  (params (DeltaSeconds :type "Float (single-precision)"))
  (bind (_returnvalue_x _returnvalue_y _returnvalue_z) (`KismetMathLibrary.BreakVector` (`self.K2_GetActorLocation`)))
  (`self.K2_SetActorLocation` (`KismetMathLibrary.MakeVector` (.x (`self.K2_GetActorLocation`)) (.y (`self.K2_GetActorLocation`)) (- (.z (`self.K2_GetActorLocation`)) (* DeltaSeconds (`self.Speed`)))))
  (`self.K2_AddActorWorldRotation` (`KismetMathLibrary.MakeRotator` 0.0 (* (`self.Speed`) 0.01)))
  (if (<= _returnvalue_z -2500.0)
    (`self.K2_DestroyActor`)))

(fn `UserConstructionScript`
  (`PaperSpriteComponent.SetSprite` (`self.PaperSprite`) (`self.Sprite`)))