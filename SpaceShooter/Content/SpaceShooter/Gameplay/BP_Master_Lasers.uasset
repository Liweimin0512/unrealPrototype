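; Base laser projectile for the space shooter that destroys what it overlaps.
; On BeginPlay it copies its Speed variable into the projectile movement component's initial speed.
; Overlaps destroy both the other actor and the laser, skipping only actors whose exact class is the player ship or this master laser.
; Tick destroys the laser once it reaches a fixed height on the Z axis.
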(event `self.ReceiveBeginPlay`
  (set `ProjectileMovementComponent.InitialSpeed` (`self.speed`) (`self.ProjectileMovement`)))

(event `self.ReceiveActorBeginOverlap`
  (params (OtherActor :type "Actor Object Reference"))
  (bind _returnvalue (`GameplayStatics.GetObjectClass` OtherActor))
  (if (and (!= _returnvalue "/Game/SpaceShooter/Gameplay/BP_PlayerShip.BP_PlayerShip_C") (!= _returnvalue "BP_Master_Lasers_C"))
    (`self.K2_DestroyActor` OtherActor)
    (`self.K2_DestroyActor`)))

(event `self.ReceiveTick`
  (params (DeltaSeconds :type "Float (single-precision)"))
  (if (>= (.z (`self.K2_GetActorLocation`)) 1250.0)
    (`self.K2_DestroyActor`)))

(fn `UserConstructionScript`)