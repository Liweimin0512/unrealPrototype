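; Scrolling background actor for the space shooter, moving continuously downward along the world Z axis.
; Tick lowers its position by Speed scaled by delta time, without sweeping.
; At or below a fixed lower Z limit it snaps back to a fixed top position, resetting X and Y to zero and discarding any overshoot.
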(event `self.ReceiveTick`
  (params (DeltaSeconds :type "Float (single-precision)"))
  (bind (_returnvalue_x _returnvalue_y _returnvalue_z) (`KismetMathLibrary.BreakVector` (`self.K2_GetActorLocation`)))
  (`self.K2_SetActorLocation` (`KismetMathLibrary.MakeVector` (.x (`self.K2_GetActorLocation`)) (.y (`self.K2_GetActorLocation`)) (- (.z (`self.K2_GetActorLocation`)) (* DeltaSeconds (`self.Speed`)))))
  (if (<= _returnvalue_z -2500.0)
    (`self.K2_SetActorLocation` (0.0 0.0 2500.0))))

(fn `UserConstructionScript`)