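; BP_Background is a background actor that scrolls continuously downward along the world Z axis in a repeating loop.
; Each Tick lowers its location by Speed scaled by delta time, leaving X and Y unchanged.
; Once it reaches the lower Z limit, it snaps to a fixed upper height, discarding any overshoot, and continues scrolling.
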(event `self.ReceiveTick`
  (params (DeltaSeconds :type "Float (single-precision)"))
  (`self.K2_SetActorLocation` (`KismetMathLibrary.MakeVector` (.x (`self.K2_GetActorLocation`)) (.y (`self.K2_GetActorLocation`)) (- (.z (`self.K2_GetActorLocation`)) (* DeltaSeconds (`self.Speed`)))))
  (if (<= (.z (`self.K2_GetActorLocation`)) -1250.0)
    (`self.K2_SetActorLocation` (`KismetMathLibrary.MakeVector` (.x (`self.K2_GetActorLocation`)) (.y (`self.K2_GetActorLocation`)) 1250.0))))

(fn `UserConstructionScript`)