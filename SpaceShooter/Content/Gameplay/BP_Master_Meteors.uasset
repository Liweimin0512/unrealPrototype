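; Master meteor actor for a space shooter that falls down world Z while spinning, with both rates driven by Speed.
; It destroys itself on reaching the lower boundary read from BP_SpaceShooterGameMode at BeginPlay.
; Sprite overlap destroys the other actor only if its class is exactly BP_Master_PlayerShip.
; Any destruction of the meteor, including at the boundary, spawns PlayerShip1_damage at its location.
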(event `self.ReceiveBeginPlay`
  (bind _asbp_space_shooter_game_mode (cast `/Game/Gameplay/BP_SpaceShooterGameMode` (`GameplayStatics.GetGameMode`)))
  (set `self.Boundary Down` (`/Game/Gameplay/BP_SpaceShooterGameMode.boundary_down` _asbp_space_shooter_game_mode)))

(event `self.ReceiveTick`
  (params (DeltaSeconds :type "Float (single-precision)"))
  (`self.K2_SetActorLocation` (`KismetMathLibrary.MakeVector` (.x (`self.K2_GetActorLocation`)) (.y (`self.K2_GetActorLocation`)) (- (.z (`self.K2_GetActorLocation`)) (* DeltaSeconds (`self.Speed`)))))
  (`self.K2_AddActorWorldRotation` (`KismetMathLibrary.MakeRotator` 0.0 (* (`self.speed`) 0.01)))
  (if (<= (.z (`self.K2_GetActorLocation`)) (`self.Boundary Down`))
    (`self.K2_DestroyActor`)))

(event `self.PaperSprite.OnComponentBeginOverlap`
  (params (OverlappedComponent :type "PrimitiveComponent Object Reference") (OtherActor :type "Actor Object Reference") (OtherComp :type "PrimitiveComponent Object Reference") (OtherBodyIndex :type Integer) (bFromSweep :type Boolean) (SweepResult :type "HitResult Structure (by ref)"))
  (if (== (`GameplayStatics.GetObjectClass` OtherActor) "/Game/Gameplay/BP_Master_PlayerShip.BP_Master_PlayerShip_C")
    (`self.K2_DestroyActor` OtherActor)))

(event `self.ReceiveDestroyed`
  (`|SpawnActorFromClass` "/Game/Gameplay/playerShip1_damage.playerShip1_damage_C" (`KismetMathLibrary.Conv_VectorToTransform` (`self.K2_GetActorLocation`)) "AlwaysSpawn" "OverrideRootScale" null null))

(fn `UserConstructionScript`)