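; BP_Master_PlayerShip is the player ship Blueprint for a Paper2D space shooter.
; On BeginPlay it registers itself as PlayerShip on BP_SpaceShooterGameMode.
; Its Launch event spawns a BP_Master_Lasers actor at the sprite's launchPosition socket.
; When destroyed, it hands the first player controller's view target to the BP_SpaceShooterCamera actor in the level.
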(event `self.ReceiveBeginPlay`
  (bind _asbp_space_shooter_game_mode (cast `/Game/Gameplay/BP_SpaceShooterGameMode` (`GameplayStatics.GetGameMode`)))
  (set `/Game/Gameplay/BP_SpaceShooterGameMode.PlayerShip` self _asbp_space_shooter_game_mode))

(event `self.ReceiveDestroyed`
  (bind _returnvalue (`GameplayStatics.GetActorOfClass` "/Game/Gameplay/BP_SpaceShooterCamera.BP_SpaceShooterCamera_C"))
  (`PlayerController.SetViewTargetWithBlend` (`GameplayStatics.GetPlayerController` 0) _returnvalue 0.0 "VTBlend_Linear" 0.0 false))

(event `Launch`
  (`|SpawnActorFromClass` "/Game/Gameplay/BP_Master_Lasers.BP_Master_Lasers_C" (`KismetMathLibrary.Conv_VectorToTransform` (`SceneComponent.GetSocketLocation` (`self.PaperSprite`) "launchPosition")) "Undefined" "OverrideRootScale" null null))

(fn `UserConstructionScript`
  (`parent.UserConstructionScript`))