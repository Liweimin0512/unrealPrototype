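; Player controller for a space shooter that spawns and drives the player ship.
; On BeginPlay it spawns BP_Master_PlayerShip at the world origin, possesses it, and switches the view target to the BP_SpaceShooterCamera found in the level.
; The "up" and "left" axes feed movement input along world Z and X scaled by the ship's Speed.
; The "launch" action calls the ship's Launch.
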(event `self.ReceiveBeginPlay`
  (bind _returnvalue (`|SpawnActorFromClass` "/Game/Gameplay/BP_Master_PlayerShip.BP_Master_PlayerShip_C" (`KismetMathLibrary.MakeTransform` (0.0 0.0 0.0)) "Undefined" "OverrideRootScale" null null))
  (bind _output_get (set `self.PlayerShip` _returnvalue))
  (`self.Possess` _output_get)
  (bind _returnvalue_2 (`GameplayStatics.GetActorOfClass` "/Game/Gameplay/BP_SpaceShooterCamera.BP_SpaceShooterCamera_C"))
  (`self.SetViewTargetWithBlend` _returnvalue_2))

(event `InputAxis|up`
  (params (AxisValue :type "Float (single-precision)"))
  (if (!= AxisValue 0.0)
    (`/Engine/EditorBlueprintResources/StandardMacros.IsValid` (`self.PlayerShip`)
      (:`Is Valid`
        (`Pawn.AddMovementInput` (`self.PlayerShip`) (`KismetMathLibrary.MakeVector` 0.0 0.0 (* AxisValue (`/Game/Gameplay/BP_Master_Ship.Speed` (`self.PlayerShip`)))) 1.0 false)))))

(event `InputAxis|left`
  (params (AxisValue :type "Float (single-precision)"))
  (if (!= AxisValue 0.0)
    (`/Engine/EditorBlueprintResources/StandardMacros.IsValid` (`self.PlayerShip`)
      (:`Is Valid`
        (`Pawn.AddMovementInput` (`self.PlayerShip`) (`KismetMathLibrary.MakeVector` (* (`/Game/Gameplay/BP_Master_Ship.Speed` (`self.PlayerShip`)) AxisValue)) 1.0 false)))))

(event `InputAction|launch`
  (params (Key :type "Key Structure"))
  (bind _playership (`self.PlayerShip`))
  (:`Pressed`
    (`/Engine/EditorBlueprintResources/StandardMacros.IsValid` _playership
      (:`Is Valid`
        (`/Game/Gameplay/BP_Master_PlayerShip.Launch` _playership)))))

(fn `UserConstructionScript`)