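; BP_BlockBase is a destructible 2D block for the Mission Demolition game, built on a Paper2D sprite component.
; On each component hit, it compares its own momentum (velocity times mass) against MaxImpact and decrements HP when that threshold is met.
; A switch on HP swaps in BrokenSprite, if valid, at one point left and destroys the actor at zero.
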(event `self.PaperSprite.OnComponentHit`
  (params (HitComponent :type "PrimitiveComponent Object Reference") (OtherActor :type "Actor Object Reference") (OtherComp :type "PrimitiveComponent Object Reference") (NormalImpulse :type "Vector Structure") (Hit :type "HitResult Structure (by ref)"))
  (bind _papersprite (`self.PaperSprite`))
  (bind _brokensprite (`self.BrokenSprite`))
  (if (>= (`KismetMathLibrary.VSize` (* (`SceneComponent.GetComponentVelocity` _papersprite) (`PrimitiveComponent.GetMass` _papersprite))) (`self.MaxImpact`))
    (bind _result (`/Engine/EditorBlueprintResources/StandardMacros.DecrementInt` (`self.HP`))
      (:`  `
        (switch `int` _result
          (:`0`
            (`self.K2_DestroyActor`))
          (:`1`
            (`/Engine/EditorBlueprintResources/StandardMacros.IsValid` _brokensprite
              (:`Is Valid`
                (`PaperSpriteComponent.SetSprite` (`self.PaperSprite`) _brokensprite)))))))))

(fn `UserConstructionScript`)