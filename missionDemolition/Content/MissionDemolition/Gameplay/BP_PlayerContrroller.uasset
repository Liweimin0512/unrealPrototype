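; Player controller for the Mission Demolition slingshot game that turns touch input into sling aiming and launching.
; On BeginPlay it sets the view target to the BP_Camera actor and caches the BP_Sling actor.
; While CanTouch is true, a press stores the viewport mouse position on the sling, moving calls Aim, and releasing calls Launch.
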(event `self.ReceiveBeginPlay`
  (bind _returnvalue (`GameplayStatics.GetActorOfClass` "/Game/MissionDemolition/Gameplay/BP_Camera.BP_Camera_C"))
  (`self.SetViewTargetWithBlend` _returnvalue)
  (bind _returnvalue_2 (`GameplayStatics.GetActorOfClass` "/Game/MissionDemolition/Sling/BP_Sling.BP_Sling_C"))
  (set `self.Sling` _returnvalue_2))

(event `InputTouch`
  (params (Location :type "Vector Structure") (FingerIndex :type "ETouchIndex Enum"))
  (:`Pressed`
    (if (`self.bCanTouch`)
      (bind _returnvalue (`WidgetLayoutLibrary.GetMousePositionOnViewport`))
      (set `/Game/MissionDemolition/Sling/BP_Sling.ClickedPostion` _returnvalue (`self.Sling`))))
  (:`Released`
    (if (`self.bCanTouch`)
      (`/Game/MissionDemolition/Sling/BP_Sling.Launch` (`self.Sling`))))
  (:`Moved`
    (if (`self.bCanTouch`)
      (`/Game/MissionDemolition/Sling/BP_Sling.Aim` (`self.Sling`)))))

(fn `UserConstructionScript`)