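; BP_Sling is the Mission Demolition slingshot that spawns, aims and launches bird projectiles.
; Aim turns the clamped mouse drag from the clicked position into an X/Z velocity, then rebuilds a trail of BP_AimBall actors along the predicted projectile path.
; Launch applies that velocity as an impulse with gravity and disables player touch.
; CreateBrid spawns a bird and re-enables touch at BeginPlay, with Launch binding bird destruction for respawning.
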(event `self.ReceiveBeginPlay`
  (`self.CreateBrid` null))

(event `self.ReceiveTick`
  (params (DeltaSeconds :type "Float (single-precision)")))

(fn `Aim`
  (bind _aimballs (`self.AimBalls`))
  (for _array_element _aimballs
    (`self.K2_DestroyActor` _array_element))
  (`KismetArrayLibrary.Array_Clear` _aimballs)
  (bind _returnvalue (`WidgetLayoutLibrary.GetMousePositionOnViewport`))
  (bind (_x _y) (`KismetMathLibrary.BreakVector2D` (- _returnvalue (`self.ClickedPostion`))))
  (bind _output_get (set `self.LaunchVelocity` (`KismetMathLibrary.MakeVector` (* (`KismetMathLibrary.FClamp` _x -80.0 0.0) -15.0) 0.0 (* (`KismetMathLibrary.FClamp` _y -0.0 50.0) 15.0))))
  (bind (_outhit _outpathpositions) (`GameplayStatics.Blueprint_PredictProjectilePath_ByTraceChannel` :`StartPos` (`SceneComponent.K2_GetComponentLocation` (`self.LaunchPotion`)) :`LaunchVelocity` _output_get :`ProjectileRadius` 10.0 :`DrawDebugTime` 1.0))
  (for _array_element_2 _outpathpositions
    (bind _returnvalue_2 (`|SpawnActorFromClass` "/Game/MissionDemolition/AimBall/BP_AimBall.BP_AimBall_C" (`KismetMathLibrary.Conv_VectorToTransform` _array_element_2) "Undefined" "OverrideRootScale" null null))
    (`KismetArrayLibrary.Array_Add` (`self.AimBalls`) _returnvalue_2)))

(fn `CreateBrid`
  (params (DestroyedActor :type "Actor Object Reference"))
  (bind _returnvalue (`|SpawnActorFromClass` "/Game/MissionDemolition/Bird/BP_Brid.BP_Brid_C" (`KismetMathLibrary.Conv_VectorToTransform` (`SceneComponent.K2_GetComponentLocation` (`self.LaunchPotion`))) "Undefined" "OverrideRootScale" null null))
  (set `self.Brid` _returnvalue)
  (bind _asbp_player_contrroller (cast `/Game/MissionDemolition/Gameplay/BP_PlayerContrroller` (`GameplayStatics.GetPlayerController` 0)))
  (set `/Game/MissionDemolition/Gameplay/BP_PlayerContrroller.bCanTouch` true _asbp_player_contrroller))

(fn `Launch`
  (bind _brid (`self.Brid`))
  (bind _asbp_player_contrroller (cast `/Game/MissionDemolition/Gameplay/BP_PlayerContrroller` (`GameplayStatics.GetPlayerController` 0)))
  (set `/Game/MissionDemolition/Gameplay/BP_PlayerContrroller.bCanTouch` false _asbp_player_contrroller)
  (set `/Game/MissionDemolition/Bird/BP_Brid.bLaunch` true _brid)
  (`PrimitiveComponent.SetEnableGravity` (`/Game/MissionDemolition/Gameplay/BP_BlockBase.PaperSprite` _brid) true)
  (`PrimitiveComponent.AddImpulse` (`/Game/MissionDemolition/Gameplay/BP_BlockBase.PaperSprite` (`self.Brid`)) (`self.LaunchVelocity`) "None" true)
  (add `self.OnDestroyed` (`self.Brid`) (`|CreateDelegate` :!event `CreateBrid`)))

(fn `UserConstructionScript`)